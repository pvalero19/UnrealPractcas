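; LightDoor is a puzzle door that opens once the counted lights match the total number of Light actors in the level.
; AddTo and RemoveFrom adjust a counter, and AddTo compares it against GetAllActorsOfClass to trigger WinningCondition.
; Winning moves the Cube to a raised relative location, sets a WIN flag and hides the HUD text.
; Until then, overlapping the actor shows a puzzle prompt through HUD_MainHUD, hidden again on exit.
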(event `AddTo`
  ;[1 1 1] Ammount Of Lights
  (set `self.int` (+ (`self.int`) 1))
  (bind _outactors (`GameplayStatics.GetAllActorsOfClass` "/Game/Blueprints/Light.Light_C"))
  (if (== (`KismetArrayLibrary.Array_Length` _outactors) (`self.int`))
    (`KismetSystemLibrary.PrintString` "WIIIN!")
    (`self.WinningCondition`)))

(event `WinningCondition`
  ;[1 1 1] OpenDoor
  (`SceneComponent.K2_SetRelativeLocation` (`self.Cube`) (0.0 0.0 200.0) false false)
  (set `self.WIN` true)
  (bind _ashud_main_hud (cast `/Game/Blueprints/Prac2/HUD_MainHUD` (`PlayerController.GetHUD` (`GameplayStatics.GetPlayerController` 0))))
  (`/Game/Blueprints/Prac2/HUD_MainHUD.ShowText_Hide` _ashud_main_hud))

(event `RemoveFrom`
  (bind _int (`self.int`))
  ;[1 1 1] Remove FRom
  (if (> _int 0)
    (set `self.int` (- _int 1))))

(event `self.ReceiveActorBeginOverlap`
  (params (OtherActor :type "Actor Object Reference"))
  ;[1 1 1] Set text to show
  (if (not (`self.WIN`))
    (bind _ashud_main_hud (cast `/Game/Blueprints/Prac2/HUD_MainHUD` (`PlayerController.GetHUD` (`GameplayStatics.GetPlayerController` 0))))
    (`/Game/Blueprints/Prac2/HUD_MainHUD.ShowText_Show` _ashud_main_hud)
    (`/Game/Blueprints/Prac2/HUD_MainHUD.ShowText_SetText` _ashud_main_hud "COMPLETE THE LIGHT PUZZLE")))

(event `self.ReceiveActorEndOverlap`
  (params (OtherActor :type "Actor Object Reference"))
  ;[1 1 1] hide text to show
  (if (not (`self.WIN`))
    (bind _ashud_main_hud (cast `/Game/Blueprints/Prac2/HUD_MainHUD` (`PlayerController.GetHUD` (`GameplayStatics.GetPlayerController` 0))))
    (`/Game/Blueprints/Prac2/HUD_MainHUD.ShowText_Hide` _ashud_main_hud)))

(fn `UserConstructionScript`)