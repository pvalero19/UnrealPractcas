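; Confusion zone that sets the Confusion flag on the player's BP_Character when its Box is overlapped, then clears it after a short time.
; Any begin overlap sets the flag on player pawn 0 and resets the TimeSec counter, without checking which actor entered.
; Tick runs a half-second Delay to increment the counter, repeatedly clearing the flag once it reaches the threshold, about 2.5 seconds later.
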(event `self.Box.OnComponentBeginOverlap`
  (params (OverlappedComponent :type "PrimitiveComponent Object Reference") (OtherActor :type "Actor Object Reference") (OtherComp :type "PrimitiveComponent Object Reference") (OtherBodyIndex :type Integer) (bFromSweep :type Boolean) (SweepResult :type "HitResult Structure (by ref)"))
  ;[1 1 1] Confusion
  (bind _asbp_character (cast `/Game/ThirdPersonBP/Blueprints/BP_Character` (`GameplayStatics.GetPlayerPawn` 0)))
  (set `/Game/ThirdPersonBP/Blueprints/BP_Character.Confusion` true _asbp_character)
  (set `self.timeSec` 0))

(event `self.ReceiveTick`
  (params (DeltaSeconds :type "Float (single-precision)"))
  ;[1 1 1] Timmer
  (`KismetSystemLibrary.Delay` 0.5)
  (set `self.timeSec` (+ (`self.timeSec`) 1))
  (if (>= (`self.timeSec`) 5)
    (bind _asbp_character (cast `/Game/ThirdPersonBP/Blueprints/BP_Character` (`GameplayStatics.GetPlayerPawn` 0)))
    (set `/Game/ThirdPersonBP/Blueprints/BP_Character.Confusion` false _asbp_character)))

(fn `UserConstructionScript`)