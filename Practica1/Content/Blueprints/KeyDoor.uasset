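; KeyDoor is a door Blueprint that opens when its trigger Box is overlapped while the player character holds at least one key.
; Opening instantly raises the Cube without consuming a key, and leaving the Box lowers it and hides the prompt.
; Each overlap creates a WID_KeyDoor widget, shown only when the key is missing.
; The overlap reads player 0's BP_Character rather than checking the overlapping actor.
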(event `self.Box.OnComponentBeginOverlap`
  (params (OverlappedComponent :type "PrimitiveComponent Object Reference") (OtherActor :type "Actor Object Reference") (OtherComp :type "PrimitiveComponent Object Reference") (OtherBodyIndex :type Integer) (bFromSweep :type Boolean) (SweepResult :type "HitResult Structure (by ref)"))
  ;[1 1 1] OpenKeyDoor
  (bind _asbp_character (cast `/Game/ThirdPersonBP/Blueprints/BP_Character` (`GameplayStatics.GetPlayerCharacter` 0)))
  ;[1 1 1] WidgetKEYDoor
  (bind _returnvalue (`|CreateWidget` "/Game/Blueprints/Prac2/WID_KeyDoor.WID_KeyDoor_C" (`GameplayStatics.GetPlayerController` 0)))
  (bind _output_get (set `self.KeyDoor` _returnvalue))
  (`UserWidget.AddToPlayerScreen` _output_get 0)
  (`Widget.SetVisibility` (`self.KeyDoor`) "Hidden")
  (if (>= (`/Game/ThirdPersonBP/Blueprints/BP_Character.Key` _asbp_character) 1)
    (`Widget.RemoveFromParent` (`self.KeyDoor`))
    (`SceneComponent.K2_SetRelativeLocation` (`self.Cube`) (0.0 0.0 200.0) false false)
    (else
      (`Widget.SetVisibility` (`self.KeyDoor`) "Visible"))))

(event `self.Box.OnComponentEndOverlap`
  (params (OverlappedComponent :type "PrimitiveComponent Object Reference") (OtherActor :type "Actor Object Reference") (OtherComp :type "PrimitiveComponent Object Reference") (OtherBodyIndex :type Integer))
  ;[1 1 1] CloseDoor
  (`Widget.SetVisibility` (`self.KeyDoor`) "Hidden")
  (`SceneComponent.K2_SetRelativeLocation` (`self.Cube`) (0.0 0.0 0.0) false false))

(fn `UserConstructionScript`)