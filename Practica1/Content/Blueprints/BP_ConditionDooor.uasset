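; BP_ConditionDooor is a door that opens permanently in exchange for a required number of coins and keys.
; On box overlap it checks the player character's inventory, then once subtracts the cost, updates the HUD counters, raises the mesh and plays a sound.
; Otherwise the main HUD shows the missing amounts, and hides them when the character leaves still short.
; Despite the CloseDoor label, end overlap never lowers the door.
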(event `self.Box.OnComponentBeginOverlap`
  (params (OverlappedComponent :type "PrimitiveComponent Object Reference") (OtherActor :type "Actor Object Reference") (OtherComp :type "PrimitiveComponent Object Reference") (OtherBodyIndex :type Integer) (bFromSweep :type Boolean) (SweepResult :type "HitResult Structure (by ref)"))
  (bind _mesh (`self.Mesh`))
  ;[1 1 1] OpenKeyDoor
  (bind _asbp_character (cast `/Game/ThirdPersonBP/Blueprints/BP_Character` (`GameplayStatics.GetPlayerCharacter` 0)))
  (if (`self.CanOpen` _asbp_character)
    (set `self.IsOpen` true))
  (if (`self.IsOpen`)
    (`/Engine/EditorBlueprintResources/StandardMacros.DoOnce` false
      (:`Completed`
        (`self.Item Substract` _asbp_character)
        (`SceneComponent.K2_SetRelativeLocation` _mesh (0.0 0.0 200.0) false false)
        (`GameplayStatics.PlaySoundAtLocation` "/Game/Blueprints/Prac2/Sounds/Door.Door" (`SceneComponent.K2_GetComponentLocation` _mesh) (struct) 1.0 1.0 0.0 null null null)))
    (else
      (bind _ashud_main_hud (cast `/Game/Blueprints/Prac2/HUD_MainHUD` (`PlayerController.GetHUD` (`GameplayStatics.GetPlayerController` 0))))
      (`/Game/Blueprints/Prac2/HUD_MainHUD.ShowText_Show` _ashud_main_hud)
      (`self.SetTextFromNeedCoinsAndKeys` _asbp_character _ashud_main_hud))))

(event `self.Box.OnComponentEndOverlap`
  (params (OverlappedComponent :type "PrimitiveComponent Object Reference") (OtherActor :type "Actor Object Reference") (OtherComp :type "PrimitiveComponent Object Reference") (OtherBodyIndex :type Integer))
  ;[1 1 1] CloseDoor
  (bind _asbp_character (cast `/Game/ThirdPersonBP/Blueprints/BP_Character` OtherActor))
  (if (not (`self.CanOpen` _asbp_character))
    (bind _ashud_main_hud (cast `/Game/Blueprints/Prac2/HUD_MainHUD` (`PlayerController.GetHUD` (`GameplayStatics.GetPlayerController` 0))))
    (`/Game/Blueprints/Prac2/HUD_MainHUD.ShowText_Hide` _ashud_main_hud)))

(fn `CanOpen`
  (params (MainCharacter :type "/Game/ThirdPersonBP/Blueprints/BP_Character Object Reference"))
  (returns (CanOpen :type Boolean))
  (return (and (>= (`/Game/ThirdPersonBP/Blueprints/BP_Character.Coins` MainCharacter) (`self.NeededCoins`)) (>= (`/Game/ThirdPersonBP/Blueprints/BP_Character.Key` MainCharacter) (`self.NeededKey`)))))

(fn `Item Substract`
  (params (BP_Character :type "/Game/ThirdPersonBP/Blueprints/BP_Character Object Reference"))
  (set `/Game/ThirdPersonBP/Blueprints/BP_Character.Key` (- (`/Game/ThirdPersonBP/Blueprints/BP_Character.Key` BP_Character) (`self.NeededKey`)) BP_Character)
  (bind _ashud_main_hud (cast `/Game/Blueprints/Prac2/HUD_MainHUD` (`PlayerController.GetHUD` (`GameplayStatics.GetPlayerController` 0))))
  (`/Game/Blueprints/Prac2/HUD_INGAME.ShowKeys` (`/Game/Blueprints/Prac2/HUD_MainHUD.IngameBase` _ashud_main_hud))
  (set `/Game/ThirdPersonBP/Blueprints/BP_Character.Coins` (- (`/Game/ThirdPersonBP/Blueprints/BP_Character.Coins` BP_Character) (`self.NeededCoins`)) BP_Character)
  (bind _ashud_main_hud_2 (cast `/Game/Blueprints/Prac2/HUD_MainHUD` (`PlayerController.GetHUD` (`GameplayStatics.GetPlayerController` 0))))
  (`/Game/Blueprints/Prac2/HUD_INGAME.ShowCoins` (`/Game/Blueprints/Prac2/HUD_MainHUD.IngameBase` _ashud_main_hud_2))
  (return))

(fn `SetTextFromNeedCoinsAndKeys`
  (params (MainCharacterRef :type "/Game/ThirdPersonBP/Blueprints/BP_Character Object Reference") (HudRef :type "/Game/Blueprints/Prac2/HUD_MainHUD Object Reference"))
  (bind _returnvalue (- (`/Game/ThirdPersonBP/Blueprints/BP_Character.Coins` MainCharacterRef) (`self.NeededCoins`)))
  (bind _returnvalue_2 (- (`/Game/ThirdPersonBP/Blueprints/BP_Character.Key` MainCharacterRef) (`self.NeededKey`)))
  (bind _output_get (set `self.Text` ""))
  (if (not (>= _returnvalue 0))
    (set `self.Text` (`KismetStringLibrary.Concat_StrStr` (`KismetStringLibrary.Concat_StrStr` " You need " (`KismetStringLibrary.Conv_IntToString` (`KismetMathLibrary.Abs_Int` _returnvalue))) " coins")))
  (if (not (>= _returnvalue_2 0))
    (set `self.Text` (`KismetStringLibrary.Concat_StrStr` (`self.Text`) (`KismetStringLibrary.Concat_StrStr` (`KismetStringLibrary.Concat_StrStr` " You need " (`KismetStringLibrary.Conv_IntToString` (`KismetMathLibrary.Abs_Int` _returnvalue_2))) " key"))))
  (`/Game/Blueprints/Prac2/HUD_MainHUD.ShowText_SetText` HudRef _output_get))

(fn `UserConstructionScript`)