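; Main HUD that builds the player's on-screen widgets and exposes helpers for prompt text and the pause menu.
; On BeginPlay it creates and stores the ShowText and in-game base widgets, with wrapper functions to show, hide and set the text.
; PauseGame opens a new pause menu and switches to UI-only input, without itself pausing the game.
; The puzzle door widget creation is disconnected and never runs.
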(event `self.ReceiveBeginPlay`
  (bind _returnvalue (`GameplayStatics.GetPlayerController` 0))
  ;[1 1 1] CreateWidgets
  (`|ExecutionSequence`
    (:`then_0`
      (bind _returnvalue_2 (`|CreateWidget` "/Game/Blueprints/Prac2/WID_ShowText.WID_ShowText_C" _returnvalue))
      (bind _output_get (set `self.ShowText` _returnvalue_2))
      (`UserWidget.AddToViewport` _output_get 0))
    (:`then_1`
      (bind _returnvalue_3 (`|CreateWidget` "/Game/Blueprints/Prac2/HUD_INGAME.HUD_INGAME_C" _returnvalue))
      (bind _output_get_2 (set `self.IngameBase` _returnvalue_3))
      (`UserWidget.AddToViewport` _output_get_2 0))))

(fn `PauseGame`
  (bind _returnvalue (`GameplayStatics.GetPlayerController` 0))
  (bind _returnvalue_2 (`|CreateWidget` "/Game/Blueprints/Prac2/MenuPausa.MenuPausa_C" _returnvalue))
  (`UserWidget.AddToPlayerScreen` _returnvalue_2 0)
  (`WidgetBlueprintLibrary.SetInputMode_UIOnlyEx` _returnvalue _returnvalue_2))

(fn `ShowText_Hide`
  (`/Game/Blueprints/Prac2/WID_ShowText.Hide` (`self.ShowText`)))

(fn `ShowText_SetText`
  (params (NewText :type String))
  (`/Game/Blueprints/Prac2/WID_ShowText.Set_Text` (`self.ShowText`) NewText))

(fn `ShowText_Show`
  (`/Game/Blueprints/Prac2/WID_ShowText.Show` (`self.ShowText`)))

(fn `UserConstructionScript`)