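; BP_PossessBullet is a projectile that triggers possession of the NPC pawn it hits.
; It moves along its local X axis each tick with a swept offset scaled by Speed, and expires after a fixed lifetime.
; On collision overlap it ignores BP_Character and non-pawns.
; Any other pawn receives a PossessNPC message carrying the first player's controller and character, then the bullet destroys itself.
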(event `self.ReceiveBeginPlay`
  (`KismetSystemLibrary.Delay` 10.0)
  (`self.K2_DestroyActor`))

(event `self.ReceiveTick`
  (params (DeltaSeconds :type "Float (single-precision)"))
  (`self.K2_AddActorLocalOffset` (`KismetMathLibrary.MakeVector` (* DeltaSeconds (`self.Speed`))) true))

(event `self.collision.OnComponentBeginOverlap`
  (params (OverlappedComponent :type "PrimitiveComponent Object Reference") (OtherActor :type "Actor Object Reference") (OtherComp :type "PrimitiveComponent Object Reference") (OtherBodyIndex :type Integer) (bFromSweep :type Boolean) (SweepResult :type "HitResult Structure (by ref)"))
  (cast `/Game/ThirdPersonBP/Blueprints/BP_Character` OtherActor
    (:`CastFailed`
      (bind _aspawn (cast `Pawn` OtherActor))
      (message `/Game/Blueprints/Prac2/Interfaces/BPI_DamageInteraction.PossessNPC` _aspawn (`GameplayStatics.GetPlayerController` 0) (`GameplayStatics.GetPlayerCharacter` 0))
      (`self.K2_DestroyActor`))))

(fn `UserConstructionScript`)