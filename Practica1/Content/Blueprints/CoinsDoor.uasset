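; CoinsDoor is a door that opens only when the player character holds at least four coins.
; Overlapping its Box creates a CoinDoor widget, then either removes it and instantly raises the Cube, or shows the widget when coins are short.
; Ending the overlap hides the widget and returns the Cube to its origin, and coins are only checked, never deducted.
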(event `self.Box.OnComponentBeginOverlap`
  (params (OverlappedComponent :type "PrimitiveComponent Object Reference") (OtherActor :type "Actor Object Reference") (OtherComp :type "PrimitiveComponent Object Reference") (OtherBodyIndex :type Integer) (bFromSweep :type Boolean) (SweepResult :type "HitResult Structure (by ref)"))
  (bind _coindoor (`self.CoinDoor`))
  ;[1 1 1] OpenKeyDoor
  (bind _ascharacter (cast `/Game/ThirdPersonBP/Blueprints/Character` (`GameplayStatics.GetPlayerCharacter` 0)))
  ;[1 1 1] WidgetCoinDoor
  (bind _returnvalue (`|CreateWidget` "/Game/Blueprints/Prac2/CoinDoor.CoinDoor_C" (`GameplayStatics.GetPlayerController` 0)))
  (bind _output_get (set `self.CoinDoor` _returnvalue))
  (`UserWidget.AddToPlayerScreen` _output_get 0)
  (`Widget.SetVisibility` (`self.CoinDoor`) "Hidden")
  (if (>= (`/Game/ThirdPersonBP/Blueprints/Character.Coins` _ascharacter) 4)
    (`Widget.RemoveFromParent` _coindoor)
    (`SceneComponent.K2_SetRelativeLocation` (`self.Cube`) (0.0 0.0 200.0) false false)
    (else
      (`Widget.SetVisibility` _coindoor "Visible"))))

(event `self.Box.OnComponentEndOverlap`
  (params (OverlappedComponent :type "PrimitiveComponent Object Reference") (OtherActor :type "Actor Object Reference") (OtherComp :type "PrimitiveComponent Object Reference") (OtherBodyIndex :type Integer))
  ;[1 1 1] CloseDoor
  (`Widget.SetVisibility` (`self.CoinDoor`) "Hidden")
  (`SceneComponent.K2_SetRelativeLocation` (`self.Cube`) (0.0 0.0 0.0) false false))

(fn `UserConstructionScript`)